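; Game mode for the 2D space shooter that tracks score and ends a level in victory or game over.
; Tick checks the target score, or elapsed time if no score target is set, to trigger level completion.
; Both endings disable the player, deactivate all spawners, save the score through the game state and show a menu via the player controller.
; Score changes use a multiplier that timed boosts raise before resetting to base.
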(event `self.ReceiveBeginPlay`
  ;[1 1 1] Initialize score multiplier to base (default = 1)
  (`self.ResetScoreMultiplier`))

(event `self.ReceiveTick`
  (params (DeltaSeconds :type "Float (single-precision)"))
  ;[1 1 1] Only check level complete if not game over or already complete
  (if (not (or (`self.IsGameOver`) (`self.IsLevelComplete`)))
    ;[1 1 1] Check if time or score win condition is achieved
    (`self.CheckLevelComplete`)))

(event `LevelComplete`
  ;[1 1 1] Set Level Complete to true
  (set `self.IsLevelComplete` true)
  (`|ExecutionSequence`
    (:`then_0`
      ;[1 1 1] Play game over sound
      (`GameplayStatics.PlaySound2D` (`self.LevelCompleteSound`)))
    (:`then_1`
      ;[1 1 1] Disable the player
      (`self.DisablePlayer`))
    (:`then_2`
      ;[1 1 1] Deactivate spawner actors
      (`self.DeactivateSpawners`))
    (:`then_3`
      ;[1 1 1] Save the current score
      (`self.SaveCurrentScore`))
    (:`then_4`
      ;[1 1 1] Show the Level Complete Menu
      (`self.ShowLevelCompleteMenu`))))

(event `GameOver`
  ;[1 1 1] Set Game Over to true
  (set `self.IsGameOver` true)
  (`|ExecutionSequence`
    (:`then_0`
      ;[1 1 1] Play game over sound
      (`GameplayStatics.PlaySound2D` (`self.GameOverSound`)))
    (:`then_1`
      ;[1 1 1] Disable the player
      (`self.DisablePlayer`))
    (:`then_2`
      ;[1 1 1] Deactivate spawner actors
      (`self.DeactivateSpawners`))
    (:`then_3`
      ;[1 1 1] Save the current score
      (`self.SaveCurrentScore`))
    (:`then_4`
      ;[1 1 1] Show the Game Over Menu
      (`self.ShowGameOverMenu`))))

(event `ActivateScoreMultiplier`
  (params (Multiplier :type Integer) (Duration :type "Float (double-precision)"))
  ;[1 1 1] Set score multiplier and reset timer
  (set `self.CurrentScoreMultiplier` Multiplier)
  (`KismetSystemLibrary.K2_SetTimer` null "DeactivateScoreMultiplier" Duration))

(event `DeactivateScoreMultiplier`
  ;[1 1 1] Resets the score multiplier to the base score multiplier
  (`self.ResetScoreMultiplier`))

(fn `ChangeScore`
  (params (Delta :type Integer))
  ;[1 1 1] Add to current score and set
  (set `self.Score` (+ (* Delta (`self.CurrentScoreMultiplier`)) (`self.Score`))))

(fn `CheckLevelComplete`
  ;[1 1 1] Check level has Complete Score
  (if (> (`self.CompleteLevelScore`) 0)
    ;[1 1 1] If true, check if score is achieved
    (if (>= (`self.Score`) (`self.CompleteLevelScore`))
      (`self.LevelComplete`))
    (else
      ;[1 1 1] Else, check if level has Complete Time
      (if (> (`self.CompleteLevelTime`) 0.0)
        ;[1 1 1] If true, check if time has elapsed
        (if (>= (`KismetSystemLibrary.GetGameTimeInSeconds`) (`self.CompleteLevelTime`))
          (`self.LevelComplete`))))))

(fn `DeactivateSpawners`
  ;[1 1 1] Loop through all BaseSpawner actors and call Deactivate Spawner for each
  (bind _outactors (`GameplayStatics.GetAllActorsOfClass` "/Game/SpaceShooter2DKit/Blueprints/Spawners/BP_BaseSpawner.BP_BaseSpawner_C"))
  (for _array_element _outactors
    (`/Game/SpaceShooter2DKit/Blueprints/Spawners/BP_BaseSpawner.DeactivateSpawner` _array_element)))

(fn `DisablePlayer`
  (`|ExecutionSequence`
    (:`then_0`
      ;[1 1 1] Disable player input
      (`self.DisableInput` (`GameplayStatics.GetPlayerCharacter` 0) (`GameplayStatics.GetPlayerController` 0)))
    (:`then_1`
      ;[1 1 1] Disable player collision
      (`PrimitiveComponent.SetCollisionEnabled` (`Character.CapsuleComponent` (`GameplayStatics.GetPlayerCharacter` 0)) "NoCollision"))))

(fn `ResetScoreMultiplier`
  ;[1 1 1] Set the currect score multiplier to base score multiplier
  (set `self.CurrentScoreMultiplier` (`self.BaseScoreMultiplier`)))

(fn `SaveCurrentScore`
  ;[1 1 1] Call Save Data with current score
  (bind _asbp_space_shooter_2dgame_state (cast `/Game/SpaceShooter2DKit/Blueprints/Game/BP_SpaceShooter2DGameState` (`GameplayStatics.GetGameState`)))
  (`/Game/SpaceShooter2DKit/Blueprints/Game/BP_SpaceShooter2DGameState.SaveData` _asbp_space_shooter_2dgame_state (`self.Score`)))

(fn `ShowGameOverMenu`
  ;[1 1 1] Instruct the player controller to show the Game Over Menu
  (`/Game/SpaceShooter2DKit/Blueprints/PlayerControllers/BP_SpaceShooter2DPlayerController.ShowGameOverMenu` (cast `/Game/SpaceShooter2DKit/Blueprints/PlayerControllers/BP_SpaceShooter2DPlayerController` (`GameplayStatics.GetPlayerController` 0) :!pure true)))

(fn `ShowLevelCompleteMenu`
  ;[1 1 1] Instruct the player controller to show the Level Complete Menu
  (`/Game/SpaceShooter2DKit/Blueprints/PlayerControllers/BP_SpaceShooter2DPlayerController.ShowLevelCompleteMenu` (cast `/Game/SpaceShooter2DKit/Blueprints/PlayerControllers/BP_SpaceShooter2DPlayerController` (`GameplayStatics.GetPlayerController` 0) :!pure true)))

(fn `UserConstructionScript`)