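; Base enemy character for the 2D space shooter, configured per Type from DT_EnemyTypes at construction or through ChangeType, which also spawns its AI controller.
; It drifts downward at randomized speeds, damages the player on collision and optionally itself.
; Looping timers with randomized intervals drive optional sideways evades and multi-point projectile fire with optional homing.
; Death disables collision and shooting, awards score, and plays a flipbook before destroying the actor.
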(event `self.ReceiveAnyDamage`
  (params (Damage :type "Float (single-precision)") (DamageType :type "DamageType Object Reference") (InstigatedBy :type "Controller Object Reference") (DamageCauser :type "Actor Object Reference"))
  ;[1 1 1] Handle damage and death
  (bind _dead (`self.TakeDamage` Damage))
  (if _dead
    (`self.HandleDeath`)))

(event `self.ReceiveBeginPlay`
  ;[1 1 1] Activate skills on BeginPlay
  (`self.ActivateShooting`)
  (`self.ActivateEvading`))

(event `self.ReceiveTick`
  (params (DeltaSeconds :type "Float (single-precision)"))
  ;[1 1 1] Move when not dead
  (if (not (`self.IsDead`))
    (`self.AddMovementInput` (`KismetMathLibrary.MakeVector` (`self.MoveSpeedX`) 0.0 (`self.MoveSpeedZ`)))))

(event `self.CapsuleComponent.OnComponentHit`
  (params (HitComponent :type "PrimitiveComponent Object Reference") (OtherActor :type "Actor Object Reference") (OtherComp :type "PrimitiveComponent Object Reference") (NormalImpulse :type "Vector Structure") (Hit :type "HitResult Structure (by ref)"))
  ;[1 1 1] Handle collision with player (deal collision damage player and inflict SelfDestructDamage to self when Dies On Collision is enabled)
  (bind _asbp_player (cast `/Game/SpaceShooter2DKit/Blueprints/Characters/Player/BP_Player` OtherActor))
  (`GameplayStatics.ApplyDamage` _asbp_player (`self.CollisionDamage`) (`self.GetController`) self)
  (if (`self.DiesOnCollision`)
    (`GameplayStatics.ApplyDamage` self (`self.SelfDestructDamage`) (`self.GetController`) self)))

(event `Evade`
  (bind _returnvalue (`KismetMathLibrary.SelectFloat` -1.0 1.0 (`KismetMathLibrary.RandomBool`)))
  ;[1 1 1] Avoid double evade
  (if (not (`self.IsEvading`))
    (set `self.IsEvading` true)
    ;[1 1 1] Change movement left or right
    (`self.ChangeXMovement` _returnvalue)
    ;[1 1 1] Wait evade duration
    (`KismetSystemLibrary.Delay` (`self.EvadeDuration`))
    ;[1 1 1] Reverse the change
    (`self.ChangeXMovement` (* _returnvalue -1.0))
    ;[1 1 1] Reset variable
    (set `self.IsEvading` false)))

(event `HandleDeath`
  (`|ExecutionSequence`
    (:`then_0`
      ;[1 1 1] Play Death sound
      (`GameplayStatics.PlaySound2D` (`self.DeathSound`)))
    (:`then_1`
      ;[1 1 1] Disable collision
      (`PrimitiveComponent.SetCollisionEnabled` (`self.CapsuleComponent`) "NoCollision"))
    (:`then_2`
      ;[1 1 1] Stop movement
      (`MovementComponent.StopMovementImmediately` (`self.CharacterMovement`)))
    (:`then_3`
      ;[1 1 1] Stop shooting
      (`self.DeactivateShooting`))
    (:`then_4`
      ;[1 1 1] Change to Death animation
      (`self.ChangeAnimation` "NewEnumerator1"))
    (:`then_5`
      ;[1 1 1] Update player score
      (`self.UpdateScore`))
    (:`then_6`
      ;[1 1 1] Play Death Animation once, then destroy actor
      (`KismetSystemLibrary.Delay` (`PaperFlipbookComponent.GetFlipbookLength` (`self.Sprite`)))
      (`self.K2_DestroyActor`))))

(fn `ActivateEvading`
  ;[1 1 1] Can the enemy evade?
  (if (`self.CanEvade`)
    ;[1 1 1] Setup timer with Min and Max delay time. Looping to keep evading
    (`KismetSystemLibrary.K2_SetTimer` null "Evade" (`KismetMathLibrary.RandomFloatInRange` (`self.MinEvadeDelay`) (`self.MaxEvadeDelay`)) true)))

(fn `ActivateHoming`
  (params (Projectile :type "/Game/SpaceShooter2DKit/Blueprints/Projectiles/BP_BaseProjectile Object Reference"))
  ;[1 1 1] Check projectile not valid
  (`/Engine/EditorBlueprintResources/StandardMacros.IsValid` Projectile
    (:`Is Valid`
      ;[1 1 1] Get player and check valid
      (bind _asbp_base_character (cast `/Game/SpaceShooter2DKit/Blueprints/Characters/BP_BaseCharacter` (`GameplayStatics.GetPlayerPawn` 0)))
      (`/Engine/EditorBlueprintResources/StandardMacros.IsValid` _asbp_base_character
        (:`Is Valid`
          (`/Game/SpaceShooter2DKit/Blueprints/Projectiles/BP_BaseProjectile.EnableHoming` Projectile _asbp_base_character))))))

(fn `ActivateShooting`
  ;[1 1 1] Can the enemy shoot?
  (if (`self.CanShoot`)
    ;[1 1 1] Setup timer with Min and Max reload time. Looping to keep shooting
    (`KismetSystemLibrary.K2_SetTimer` null "Fire" (`KismetMathLibrary.RandomFloatInRange` (`self.MinReloadTime`) (`self.MaxReloadTime`)) true)))

(fn `ChangeAnimation`
  (params (AnimationState :type "/Game/SpaceShooter2DKit/Blueprints/Characters/ENUM_AnimationStates Enum" :default "NewEnumerator0"))
  (bind _animations (`self.Animations`))
  ;[1 1 1] Pick correct animation
  (switch `/Game/SpaceShooter2DKit/Blueprints/Characters/ENUM_AnimationStates` AnimationState
    (:`NewEnumerator0`
      ;[1 1 1] Set flipbook and scale
      (`self.ChangeFlipbook` (break `/Game/SpaceShooter2DKit/Blueprints/Characters/STR_Animation` (break `/Game/SpaceShooter2DKit/Blueprints/Characters/STR_AnimationProperties` _animations)) (`.Scale_5_2A52AD4EF048F88B00870499459475C5` (break `/Game/SpaceShooter2DKit/Blueprints/Characters/STR_Animation` (break `/Game/SpaceShooter2DKit/Blueprints/Characters/STR_AnimationProperties` _animations)))))
    (:`NewEnumerator1`
      (`self.ChangeFlipbook` (break `/Game/SpaceShooter2DKit/Blueprints/Characters/STR_Animation` (`.DeadAnimation_7_CCC32E6F2A427A9BAC2FCF9652C232DB` (break `/Game/SpaceShooter2DKit/Blueprints/Characters/STR_AnimationProperties` _animations))) (`.Scale_5_2A52AD4EF048F88B00870499459475C5` (break `/Game/SpaceShooter2DKit/Blueprints/Characters/STR_Animation` (`.DeadAnimation_7_CCC32E6F2A427A9BAC2FCF9652C232DB` (break `/Game/SpaceShooter2DKit/Blueprints/Characters/STR_AnimationProperties` _animations))))))))

(fn `ChangeType`
  (params (Type :type "/Game/SpaceShooter2DKit/Blueprints/Characters/Enemies/ENUM_EnemyType Enum" :default "NewEnumerator0"))
  ;[1 1 1] Set new type
  (set `self.Type` Type)
  ;[1 1 1] Load properties from Data Table
  (`self.LoadDataTableProperties`)
  ;[1 1 1] Setup enemy using loaded properties
  (`self.SetupProperties`)
  ;[1 1 1] Setup skills
  (`self.ActivateShooting`)
  (`self.ActivateEvading`)
  ;[1 1 1] Spawn AI
  (`self.SpawnAI`))

(fn `ChangeXMovement`
  (params (Delta :type "Float (double-precision)"))
  ;[1 1 1] Update the x movement speed by delta
  (set `self.MoveSpeedX` (+ (`self.MoveSpeedX`) Delta)))

(fn `DeactivateShooting`
  ;[1 1 1] Clear the Timer for Fire function
  (`KismetSystemLibrary.K2_ClearTimer` null "Fire"))

(fn `Fire`
  (bind _projectilespawnpoints_spawnpoints (break `/Game/SpaceShooter2DKit/Blueprints/Projectiles/STR_ProjectileSpawnPointGroup` (`self.ProjectileSpawnPoints`)))
  ;[1 1 1] Loop through projectile spawn points
  (for _array_element _projectilespawnpoints_spawnpoints
    ;[1 1 1] Spawn projectiles
    (bind _returnvalue (`|SpawnActorFromClass` "/Game/SpaceShooter2DKit/Blueprints/Projectiles/BP_EnemyProjectile.BP_EnemyProjectile_C" (`KismetMathLibrary.ComposeTransforms` _array_element (`SceneComponent.K2_GetComponentToWorld` (`self.CapsuleComponent`))) "Undefined" "OverrideRootScale" null null))
    ;[1 1 1] Activate homing if enabled
    (if (`self.HomingProjectiles`)
      (`self.ActivateHoming` _returnvalue))))

(fn `HasType`
  (params (Type :type "/Game/SpaceShooter2DKit/Blueprints/Characters/Enemies/ENUM_EnemyType Enum" :default "NewEnumerator0"))
  (returns (IsType :type Boolean))
  ;[1 1 1] Compare type and return
  (return (`|EnumEquality` Type (`self.Type`))))

(fn `LoadDataTableProperties`
  (bind _returnvalue (`|GetEnumeratorNameAsString` (`self.Type`)))
  ;[1 1 1] Get properties from Data Table using type variable
  (bind _returnvalue_2 (`|GetDataTableRow` "/Game/SpaceShooter2DKit/Blueprints/Characters/Enemies/DT_EnemyTypes.DT_EnemyTypes" (`KismetStringLibrary.Conv_StringToName` _returnvalue))
    (:`then`
      ;[1 1 1] If found, set properties
      (set `self.Properties` _returnvalue_2))
    (:`RowNotFound`
      ;[1 1 1] Else, display error message
      (`KismetSystemLibrary.PrintString` (`KismetStringLibrary.Concat_StrStr` _returnvalue "NOT FOUND")))))

(fn `SetCapsuleSize`
  (params (HalfHeight :type "Float (double-precision)") (Radius :type "Float (double-precision)"))
  (bind _capsulecomponent (`self.CapsuleComponent`))
  ;[1 1 1] Setup Capsule Component Dimensions, Radius first due to constrain on Half Height
  (`|ExecutionSequence`
    (:`then_0`
      (`CapsuleComponent.SetCapsuleRadius` _capsulecomponent Radius true))
    (:`then_1`
      (`CapsuleComponent.SetCapsuleHalfHeight` _capsulecomponent HalfHeight true))))

(fn `SetMoveSpeedX`
  (params (Min :type "Float (double-precision)") (Max :type "Float (double-precision)"))
  ;[1 1 1] Pick random float between min and max and set value
  (set `self.MoveSpeedX` (`KismetMathLibrary.RandomFloatInRange` Min Max)))

(fn `SetMoveSpeedZ`
  (params (Min :type "Float (double-precision)") (Max :type "Float (double-precision)"))
  ;[1 1 1] Pick random float between min and max, negate (since enemies fly down) and set value
  (set `self.MoveSpeedZ` (* (`KismetMathLibrary.RandomFloatInRange` Min Max) -1.0)))

(fn `SetRotation`
  (params (Min :type "Float (double-precision)") (Max :type "Float (double-precision)"))
  ;[1 1 1] Pick random float between min and max and set value
  (set `RotatingMovementComponent.RotationRate` (`KismetMathLibrary.MakeRotator` 0.0 (`KismetMathLibrary.RandomFloatInRange` Min Max)) (`self.RotatingMovement`)))

(fn `SetupAIProperties`
  (params (AIProperties :type "/Game/SpaceShooter2DKit/Blueprints/Characters/Enemies/STR_EnemyAIProperties Structure"))
  (set `self.AIControllerClass` AIProperties_AIController_3_7E2DD3364AC7B24B5DC300B7525B9731))

(fn `SetupBasicProperties`
  (params (BasicProperties :type "/Game/SpaceShooter2DKit/Blueprints/Characters/Enemies/STR_EnemyBasicProperties Structure"))
  (`|ExecutionSequence`
    (:`then_0`
      ;[1 1 1] Set animations variable
      (set `self.Animations` BasicProperties_Animations_34_DA78700BBE4397AFC1A73DB2211FB496))
    (:`then_1`
      ;[1 1 1] Set collision size
      (`self.SetCapsuleSize` BasicProperties_CollisionCapsuleHalfHeight_11_903ACB0AF649483F3D2017AEFD147F2D BasicProperties_CollisionCapsuleRadius_12_AC45A980254B7171D0967EB625E543F8))
    (:`then_2`
      ;[1 1 1] Set visuals
      (`self.SetVisuals` BasicProperties_Material_21_FCD659700E449E24DC82EF86CEDDEACC))
    (:`then_3`
      ;[1 1 1] Setup Health, Collision settings and Score
      (`self.UpdateMaxHealth` BasicProperties_Health_28_ED58F6B64A4A67019C62E0A24D0F75D4 true))
    (:`then_4`
      (set `self.CollisionDamage` BasicProperties_CollisionDamage_14_6B99E0D9EF4C3F0B70E651A1BC472801))
    (:`then_5`
      (set `self.DiesOnCollision` BasicProperties_DiesOnCollision_37_EA01B6DE48400F3E5BAF628EB103AB5E))
    (:`then_6`
      (set `self.Score` BasicProperties_Score_5_789A102BC64469D4362CA69CBB38C344))))

(fn `SetupEvadeProperties`
  (params (EvadeProperties :type "/Game/SpaceShooter2DKit/Blueprints/Characters/Enemies/STR_EnemyEvadeProperties Structure"))
  (`|ExecutionSequence`
    (:`then_0`
      (set `self.CanEvade` EvadeProperties_CanEvade_16_AEF4DBAFDB40D4C0E8C770B50D4AAE79))
    (:`then_1`
      (set `self.InitialEvadeDelay` EvadeProperties_InitialEvadeDelay_17_DCFF6F081947C0DB0F6C43BF1DBE2639))
    (:`then_2`
      (set `self.MinEvadeDelay` EvadeProperties_MinEvadeDelay_22_5324E9844E47AC58CE24A69B565D7D78))
    (:`then_3`
      (set `self.MaxEvadeDelay` EvadeProperties_MaxEvadeDelay_19_095C13D4AD474F92D07E0D9D20232C50))
    (:`then_4`
      (set `self.EvadeDuration` EvadeProperties_EvadeDuration_20_C0738575C04C560FD681548EF9417462))))

(fn `SetupMovementProperties`
  (params (MovementProperties :type "/Game/SpaceShooter2DKit/Blueprints/Characters/Enemies/STR_EnemyMovementProperties Structure"))
  (`|ExecutionSequence`
    (:`then_0`
      ;[1 1 1] Setup movement speed in X direction
      (`self.SetMoveSpeedX` MovementProperties_MinMoveSpeedX_7_C98F8B059F4ED2807A8173A56DEE7F02 MovementProperties_MaxMoveSpeedX_13_B66FC02BED48BBF1AAA4508337BD67BF))
    (:`then_1`
      ;[1 1 1] Setup movement speed in Z direction
      (`self.SetMoveSpeedZ` MovementProperties_MinMoveSpeedZ_14_01A91873C745E79E216570927503ECB0 MovementProperties_MaxMoveSpeedZ_15_CEF378F08C437C93454156A0B50C5DB7))
    (:`then_2`
      ;[1 1 1] Setup rotation movement
      (`self.SetRotation` MovementProperties_MinRotationRate_19_4E0F5382104D0C255C9EC9B9A9A05418 MovementProperties_MaxRotationRate_21_5F30D3C3C345FCC7C7E6A196635EF941))))

(fn `SetupProperties`
  (bind (_properties_basicproperties _properties_movementproperties _properties_shootingproperties _properties_evadeproperties _properties_soundproperties _properties_aiproperties) (break `/Game/SpaceShooter2DKit/Blueprints/Characters/Enemies/STR_EnemyProperties` (`self.Properties`)))
  (`|ExecutionSequence`
    (:`then_0`
      (`self.SetupBasicProperties` _properties_basicproperties))
    (:`then_1`
      (`self.SetupMovementProperties` _properties_movementproperties))
    (:`then_2`
      (`self.SetupShootingProperties` _properties_shootingproperties))
    (:`then_3`
      (`self.SetupEvadeProperties` _properties_evadeproperties))
    (:`then_4`
      (`self.SetupSoundProperties` _properties_soundproperties))
    (:`then_5`
      (`self.SetupAIProperties` _properties_aiproperties))))

(fn `SetupShootingProperties`
  (params (ShootingProperties :type "/Game/SpaceShooter2DKit/Blueprints/Characters/Enemies/STR_EnemyShootProperties Structure"))
  (`|ExecutionSequence`
    (:`then_0`
      (set `self.CanShoot` ShootingProperties_CanShoot_14_88D1FEC4054C6F74414F988BBA38D076))
    (:`then_1`
      (set `self.ProjectileSpawnPoints` ShootingProperties_ProjectileSpawnPoints_12_71664EFB8B4A88C9A5F4E1B9CCF2DD01))
    (:`then_2`
      (set `self.MinReloadTime` ShootingProperties_MinReloadTime_10_3EE78FFB6C4D49C4BBCF68925E4C20B2))
    (:`then_3`
      (set `self.MaxReloadTime` ShootingProperties_MaxReloadTime_11_C46019F1C6460D370311059FC24B6CC5))
    (:`then_4`
      (set `self.HomingProjectiles` ShootingProperties_HomingProjectiles_18_FE5CB7FC2040C16890087EA15E787D89))))

(fn `SetupSoundProperties`
  (params (SoundProperties :type "/Game/SpaceShooter2DKit/Blueprints/Characters/Enemies/STR_EnemySoundProperties Structure"))
  (set `self.DeathSound` SoundProperties_DeathSound_5_442E26406740A895BF2B5BB2B5252D71))

(fn `SetVisuals`
  (params (Material :type "MaterialInstance Object Reference"))
  (`|ExecutionSequence`
    (:`then_0`
      ;[1 1 1] Setup alive animation
      (`self.ChangeAnimation` "NewEnumerator0"))
    (:`then_1`
      ;[1 1 1] Setup material
      (`PrimitiveComponent.SetMaterial` (`self.Sprite`) 0 Material))))

(fn `SpawnAI`
  ;[1 1 1] Spawn AI class (location irrelevant)
  (bind _returnvalue (`|SpawnActorFromClass` (`self.AIControllerClass`) (`KismetMathLibrary.MakeTransform` (0.0 0.0 0.0)) "Undefined" "OverrideRootScale" null null))
  ;[1 1 1] Let AI posess this enemy
  (`Controller.Possess` _returnvalue self))

(fn `UpdateScore`
  ;[1 1 1] Get 2DSpaceShooter GameMode
  (bind _asbp_space_shooter_2dgame_mode (cast `/Game/SpaceShooter2DKit/Blueprints/Game/BP_SpaceShooter2DGameMode` (`GameplayStatics.GetGameMode`)))
  ;[1 1 1] Change score
  (`/Game/SpaceShooter2DKit/Blueprints/Game/BP_SpaceShooter2DGameMode.ChangeScore` _asbp_space_shooter_2dgame_mode (`self.Score`)))

(fn `UserConstructionScript`
  ;[1 1 1] Call constructor script of BaseCharacter
  (`parent.UserConstructionScript`)
  ;[1 1 1] Load properties from Data Table
  (`self.LoadDataTableProperties`)
  ;[1 1 1] Setup enemy with loaded properties
  (`self.SetupProperties`))