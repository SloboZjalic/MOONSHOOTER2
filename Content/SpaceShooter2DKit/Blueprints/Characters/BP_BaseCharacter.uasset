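; Base character Blueprint for the 2D space shooter kit, providing health, death checks, regeneration and sprite flipbook swapping.
; Health starts at max on construction; TakeDamage halts regen, subtracts clamped damage and returns whether the character is dead.
; If it survives and can regen, a delayed timer starts a looping timer that heals by passing a negative delta to SubtractHealth.
; Helpers update max health with optional refill and change the flipbook and its scale.
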(fn `ChangeFlipbook`
  (params (Flipbook :type "PaperFlipbook Object Reference") (FlipbookScale :type "Vector Structure"))
  (bind _sprite (`self.Sprite`))
  (`|ExecutionSequence`
    (:`then_0`
      ;[1 1 1] Change the flipbook
      (`PaperFlipbookComponent.SetFlipbook` _sprite Flipbook))
    (:`then_1`
      ;[1 1 1] Set its scale
      (`SceneComponent.SetRelativeScale3D` _sprite FlipbookScale))))

(fn `CheckDead`
  (returns (Dead :type Boolean))
  ;[1 1 1] Set and result value
  (bind _output_get (set `self.IsDead` (<= (`self.CurrentHealth`) 0.0)))
  (return _output_get))

(fn `InitializeHealth`
  ;[1 1 1] Set the Current Health to Max Health
  (set `self.CurrentHealth` (`self.MaxHealth`)))

(fn `RegenHealth`
  ;[1 1 1] Add regen amount to current health
  (`self.SubtractHealth` (* (`self.RegenAmount`) -1.0)))

(fn `StartHealthRegen`
  ;[1 1 1] Call RegenHealth every Regen Rate
  (`KismetSystemLibrary.K2_SetTimer` null "RegenHealth" (`self.RegenRate`) true))

(fn `StopHealthRegen`
  ;[1 1 1] Stop the start timer
  (`KismetSystemLibrary.K2_ClearTimer` null "StartHealthRegen")
  ;[1 1 1] Stop the current regen
  (`KismetSystemLibrary.K2_ClearTimer` null "RegenHealth"))

(fn `SubtractHealth`
  (params (Delta :type "Float (double-precision)"))
  ;[1 1 1] Clamp new value between 0 and Max Health
  (set `self.CurrentHealth` (`KismetMathLibrary.FClamp` (- (`self.CurrentHealth`) Delta) 0.0 (`self.MaxHealth`))))

(fn `TakeDamage`
  (params (Damage :type "Float (double-precision)"))
  (returns (Dead :type Boolean))
  ;[1 1 1] Stop health regen
  (`self.StopHealthRegen`)
  ;[1 1 1] Subtract damage
  (`self.SubtractHealth` Damage)
  ;[1 1 1] Check dead
  (bind _dead (`self.CheckDead`))
  ;[1 1 1] If true, return value. Else start health regen and return value
  (if _dead
    (return _dead)
    (else
      ;[1 1 1] Can this actor regen health?
      (if (`self.CanRegen`)
        ;[1 1 1] Start health regen after regen delay
        (`KismetSystemLibrary.K2_SetTimer` null "StartHealthRegen" (`self.RegenDelay`))
        (return _dead)))))

(fn `UpdateMaxHealth`
  (params (NewMaxHealth :type "Float (double-precision)") (FullHealth :type Boolean))
  ;[1 1 1] Set new value
  (set `self.MaxHealth` NewMaxHealth)
  ;[1 1 1] Check Full Health variable and conditionally set current health to max health
  (if FullHealth
    (set `self.CurrentHealth` (`self.MaxHealth`))))

(fn `UserConstructionScript`
  ;[1 1 1] Set initial health value
  (`self.InitializeHealth`))