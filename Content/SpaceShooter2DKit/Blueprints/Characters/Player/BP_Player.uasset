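; Player ship character for the 2D space shooter, handling movement, weapons, nukes, a one-hit shield and a slow-motion death that triggers game over.
; Ship visuals and upgradeable weapon spawn patterns come from DataTables, with the ship selected in the GameInstance.
; Firing supports tap, timer-driven hold or automatic modes with optional ammo limits.
; Movement is either physics input or swept Tick offsets, and nukes damage every enemy.
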(event `self.ReceiveAnyDamage`
  (params (Damage :type "Float (single-precision)") (DamageType :type "DamageType Object Reference") (InstigatedBy :type "Controller Object Reference") (DamageCauser :type "Actor Object Reference"))
  ;[1 1 1] Check if shield is active
  (if (`self.ShieldActive`)
    ;[1 1 1] If active, ignore the hit and deactivate shield
    (`self.DeactivateShield`)
    (else
      ;[1 1 1] Else, play hit sound and handle damage
      (`GameplayStatics.PlaySound2D` (`self.HitSound`))
      (bind _dead (`self.TakeDamage` Damage))
      ;[1 1 1] Check dead and handle if true
      (if _dead
        (`self.HandleDeath`)))))

(event `self.ReceiveBeginPlay`
  ;[1 1 1] Save Game Mode in variable
  (`self.SetGameMode`)
  ;[1 1 1] Save Player Controller in variable
  (`self.SetPlayerController`)
  ;[1 1 1] Set player ship visuals
  (`self.SetPlayerShipVisuals`)
  ;[1 1 1] Set weapon types variable and current weapon
  (`self.InitializeWeaponTypes`)
  ;[1 1 1] If not unlimited ammo, initialize ammo amount
  (if (not (`self.UnlimitedAmmo`))
    (`self.InitializeWeaponAmmo`))
  ;[1 1 1] Start firing for Automatic Fire Mode only on TestMap (not Main Menu)
  (if (`|EnumEquality` (`self.CurrentFireMode`) "NewEnumerator2")
    (bind _returnvalue (`GameplayStatics.GetCurrentLevelName` true))
    (if (`KismetStringLibrary.EqualEqual_StrStr` _returnvalue "TestMap")
      (`self.StartFiring`))))

(event `HandleDeath`
  (`|ExecutionSequence`
    (:`then_0`
      ;[1 1 1] Stop firing projectiles
      (`self.StopFiring`))
    (:`then_1`
      ;[1 1 1] Slow down time for death animation
      (`GameplayStatics.SetGlobalTimeDilation` 0.4)
      ;[1 1 1] Play dead animation once and hide player after
      (`self.ChangeAnimation` "NewEnumerator1")
      (`KismetSystemLibrary.Delay` (`PaperFlipbookComponent.GetFlipbookLength` (`self.Sprite`)))
      (`self.SetActorHiddenInGame` true)
      ;[1 1 1] Reset time dilation
      (`GameplayStatics.SetGlobalTimeDilation` 1.0))
    (:`then_2`
      ;[1 1 1] Set Game Over
      (`/Game/SpaceShooter2DKit/Blueprints/Game/BP_SpaceShooter2DGameMode.GameOver` (`self.GameMode`)))))

(event `InputAction|Fire`
  (params (Key :type "Key Structure"))
  ;[1 1 1] Handle Fire
  (:`Pressed`
    (`self.FirePressed`))
  (:`Released`
    (`self.FireReleased`)))

(event `self.ReceiveTick`
  (params (DeltaSeconds :type "Float (single-precision)"))
  (bind _gamemode (`self.GameMode`))
  ;[1 1 1] Non-physics movement using event tick and Add World Offset (only when game is not over or level complete)
  (if (`self.PhysicsMovement`)
    _
    (elif (not (or (`/Game/SpaceShooter2DKit/Blueprints/Game/BP_SpaceShooter2DGameMode.IsGameOver` _gamemode) (`/Game/SpaceShooter2DKit/Blueprints/Game/BP_SpaceShooter2DGameMode.IsLevelComplete` _gamemode)))
      (`self.NonPhysicsMovement` DeltaSeconds))))

(event `InputAction|Nuke`
  (params (Key :type "Key Structure"))
  ;[1 1 1] Handle Nuke
  (:`Pressed`
    (`self.ActivateNuke`)))

(event `InputAxis|MoveRight`
  (params (AxisValue :type "Float (single-precision)"))
  ;[1 1 1] Physics movement using Add Movement Input function
  (if (`self.PhysicsMovement`) :!label _label
    (`self.AddMovementInput` (`KismetMathLibrary.MakeVector` AxisValue 0.0 (stale `InputAxis|MoveForward` AxisValue)))))

(event `InputAction|WeaponUp`
  (params (Key :type "Key Structure"))
  ;[1 1 1] Handle Weapon Up/Down
  (:`Pressed`
    (`self.UpgradeWeapon`)))

(event `InputAxis|MoveForward`
  (params (AxisValue :type "Float (single-precision)"))
  ;[1 1 1] Physics movement using Add Movement Input function
  (goto _label))

(event `InputAction|WeaponDown`
  (params (Key :type "Key Structure"))
  ;[1 1 1] Handle Weapon Up/Down
  (:`Pressed`
    (`self.DowngradeWeapon`)))

(event `FirePressed`
  ;[1 1 1] Fire once for tap, start and release for hold, automatic handled in Event Graph on Event Begin Play
  (switch `/Game/SpaceShooter2DKit/Blueprints/Characters/Player/ENUM_FireModes` (`self.CurrentFireMode`)
    (:`NewEnumerator0`
      (`self.FireWeapon`))
    (:`NewEnumerator1`
      (`/Engine/EditorBlueprintResources/StandardMacros.DoOnce` false :!label _label
        (:`Completed`
          (`self.FireWeapon`)
          (`self.StartFiring`))))))

(event `FireReleased`
  ;[1 1 1] Fire once for tap, start and release for hold, automatic handled in Event Graph on Event Begin Play
  (if (`|EnumEquality` (`self.CurrentFireMode`) "NewEnumerator1")
    (`self.StopFiring`)
    (goto _label :!via `Reset`)))

(event `StartFiring`
  ;[1 1 1] Continiously fire weapon with fire rate
  (`KismetSystemLibrary.K2_SetTimer` null "FireWeapon" (/ 1.0 (`self.Fire rate`)) true))

(event `StopFiring`
  ;[1 1 1] Stop firing weapon
  (`KismetSystemLibrary.K2_ClearTimer` null "FireWeapon"))

(fn `ActivateNuke`
  ;[1 1 1] Check if nuke ammo is present
  (if (`self.CheckNukeAmmo`)
    ;[1 1 1] Reduce ammo with 1
    (`self.ChangeNukeAmmo` -1)
    ;[1 1 1] Loop through all enemies
    (bind _outactors (`GameplayStatics.GetAllActorsOfClass` "/Game/SpaceShooter2DKit/Blueprints/Characters/Enemies/BP_BaseEnemy.BP_BaseEnemy_C"))
    (for _array_element _outactors
      ;[1 1 1] Apply nuke damage to each enemy
      (`GameplayStatics.ApplyDamage` _array_element (`self.NukeDamage`) (`self.PlayerController`) self))))

(fn `ActivateShield`
  ;[1 1 1] Check variable and set active when inactive
  (if (not (`self.ShieldActive`))
    (set `self.ShieldActive` true)
    ;[1 1 1] Play shield up sound
    (`GameplayStatics.PlaySound2D` (`self.ShieldUpSound`))
    ;[1 1 1] Show shield sprite
    (`SceneComponent.SetVisibility` (`self.ShieldSprite`) true false)))

(fn `AddNuke`
  (`self.ChangeNukeAmmo` 1))

(fn `AddWeaponAmmo`
  (params (Amount :type Integer))
  (`self.ChangeWeaponAmmo` Amount))

(fn `ChangeAnimation`
  (params (AnimationState :type "/Game/SpaceShooter2DKit/Blueprints/Characters/ENUM_AnimationStates Enum" :default "NewEnumerator0"))
  (bind _animations (`self.Animations`))
  ;[1 1 1] Pick correct animation
  (switch `/Game/SpaceShooter2DKit/Blueprints/Characters/ENUM_AnimationStates` AnimationState
    (:`NewEnumerator0`
      ;[1 1 1] Set flipbook and scale
      (`self.ChangeFlipbook` (break `/Game/SpaceShooter2DKit/Blueprints/Characters/STR_Animation` (break `/Game/SpaceShooter2DKit/Blueprints/Characters/STR_AnimationProperties` _animations)) (`.Scale_5_2A52AD4EF048F88B00870499459475C5` (break `/Game/SpaceShooter2DKit/Blueprints/Characters/STR_Animation` (break `/Game/SpaceShooter2DKit/Blueprints/Characters/STR_AnimationProperties` _animations))))
      ;[1 1 1] Set thrusters visibility
      (`self.ToggleThrustersVisibility` true))
    (:`NewEnumerator1`
      (`self.ChangeFlipbook` (break `/Game/SpaceShooter2DKit/Blueprints/Characters/STR_Animation` (`.DeadAnimation_7_CCC32E6F2A427A9BAC2FCF9652C232DB` (break `/Game/SpaceShooter2DKit/Blueprints/Characters/STR_AnimationProperties` _animations))) (`.Scale_5_2A52AD4EF048F88B00870499459475C5` (break `/Game/SpaceShooter2DKit/Blueprints/Characters/STR_Animation` (`.DeadAnimation_7_CCC32E6F2A427A9BAC2FCF9652C232DB` (break `/Game/SpaceShooter2DKit/Blueprints/Characters/STR_AnimationProperties` _animations)))))
      (`self.ToggleThrustersVisibility` false))))

(fn `ChangeNukeAmmo`
  (params (Delta :type Integer))
  (set `self.CurrentNukeAmmo` (`KismetMathLibrary.Clamp` (+ (`self.CurrentNukeAmmo`) Delta) 0 (`self.MaxNukeAmmo`))))

(fn `ChangeWeapon`
  (params (Delta :type Integer))
  ;[1 1 1] Set the new Weapon Type Index
  (bind _output_get (set `self.WeaponTypeIndex` (+ (`self.WeaponTypeIndex`) Delta)))
  ;[1 1 1] Set the weapon type
  (`self.SetWeaponType` (`KismetMathLibrary.Clamp` _output_get 0 (- (`KismetArrayLibrary.Array_Length` (`self.WeaponTypeNames`)) 1))))

(fn `ChangeWeaponAmmo`
  (params (Delta :type Integer))
  (set `self.CurrentWeaponAmmo` (`KismetMathLibrary.Clamp` (+ (`self.CurrentWeaponAmmo`) Delta) 0 (`self.MaxWeaponAmmo`))))

(fn `CheckNukeAmmo`
  (returns (Result :type Boolean))
  (return (> (`self.CurrentNukeAmmo`) 0)))

(fn `CheckWeaponAmmo`
  (returns (HasAmmo :type Boolean))
  (locals (Result :type Boolean :default false))
  (return (select `bool` (`self.UnlimitedAmmo`) :`false` (> (`self.CurrentWeaponAmmo`) 0) :`true` true)))

(fn `DeactivateShield`
  ;[1 1 1] Reset variable
  (set `self.ShieldActive` false)
  ;[1 1 1] Play shield down sound
  (`GameplayStatics.PlaySound2D` (`self.ShieldDownSound`))
  ;[1 1 1] Hide shield sprite
  (`SceneComponent.SetVisibility` (`self.ShieldSprite`) false false))

(fn `DowngradeWeapon`
  (`self.ChangeWeapon` -1))

(fn `FireWeapon`
  (bind _currentweapontype_spawnpoints (break `/Game/SpaceShooter2DKit/Blueprints/Projectiles/STR_ProjectileSpawnPointGroup` (`self.CurrentWeaponType`)))
  (if (`self.UnlimitedAmmo`)
    ;[1 1 1] Loop through projectile spawn points
    (for _array_element _currentweapontype_spawnpoints :!label _label
      ;[1 1 1] Spawn projectiles
      (`|SpawnActorFromClass` "/Game/SpaceShooter2DKit/Blueprints/Projectiles/BP_PlayerProjectile.BP_PlayerProjectile_C" (`KismetMathLibrary.ComposeTransforms` _array_element (`SceneComponent.K2_GetComponentToWorld` (`self.CapsuleComponent`))) "Undefined" "OverrideRootScale" null null))
    ;[1 1 1] When done, play fire sound
    (`GameplayStatics.PlaySound2D` (`self.FireSound`))
    (else
      ;[1 1 1] Only fire if there is ammo
      (if (`self.CheckWeaponAmmo`)
        ;[1 1 1] Reduce ammo with 1
        (`self.ChangeWeaponAmmo` -1)
        (goto _label)))))

(fn `InitializeWeaponAmmo`
  (set `self.CurrentWeaponAmmo` (`self.BaseWeaponAmmo`)))

(fn `InitializeWeaponTypes`
  ;[1 1 1] Save the Data Table names
  (bind _outrownames (`DataTableFunctionLibrary.GetDataTableRowNames` "/Game/SpaceShooter2DKit/Blueprints/Characters/Player/DT_PlayerWeaponTypes.DT_PlayerWeaponTypes"))
  (set `self.WeaponTypeNames` _outrownames)
  ;[1 1 1] Set the current weapon type to SingleShot
  (bind _returnvalue (`|GetDataTableRow` "/Game/SpaceShooter2DKit/Blueprints/Characters/Player/DT_PlayerWeaponTypes.DT_PlayerWeaponTypes" "SingleShot")
    (:`then`
      (set `self.CurrentWeaponType` _returnvalue))))

(fn `NonPhysicsMovement`
  (params (DeltaSeconds :type "Float (double-precision)"))
  ;[1 1 1] Apply vector to location
  (`self.K2_AddActorWorldOffset` (* (`KismetMathLibrary.ClampVectorSize` (`KismetMathLibrary.MakeVector` (`self.GetInputAxisValue`) 0.0 (`self.GetInputAxisValue`)) 0.0 1.0) (* DeltaSeconds (`self.NonPhysicsMovementSpeed`))) true))

(fn `SetGameMode`
  ;[1 1 1] Get the game mode and save in variable
  (bind _asbp_space_shooter_2dgame_mode (cast `/Game/SpaceShooter2DKit/Blueprints/Game/BP_SpaceShooter2DGameMode` (`GameplayStatics.GetGameMode`)))
  (set `self.GameMode` _asbp_space_shooter_2dgame_mode))

(fn `SetPlayerController`
  ;[1 1 1] Get the player controller and save in variable
  (bind _asbp_space_shooter_2dplayer_controller (cast `/Game/SpaceShooter2DKit/Blueprints/PlayerControllers/BP_SpaceShooter2DPlayerController` (`GameplayStatics.GetPlayerController` 0)))
  (set `self.PlayerController` _asbp_space_shooter_2dplayer_controller))

(fn `SetPlayerShipVisuals`
  ;[1 1 1] Get selected player shp from Game Instance
  (bind _asbp_space_shooter_2dgame_instance (cast `/Game/SpaceShooter2DKit/Blueprints/Game/BP_SpaceShooter2DGameInstance` (`GameplayStatics.GetGameInstance`)))
  (bind _returnvalue (`|GetDataTableRow` "/Game/SpaceShooter2DKit/Blueprints/Characters/Player/DT_PlayerShips.DT_PlayerShips" (`/Game/SpaceShooter2DKit/Blueprints/Game/BP_SpaceShooter2DGameInstance.SelectedShip` _asbp_space_shooter_2dgame_instance))
    (:`then`
      (`|ExecutionSequence`
        (:`then_0`
          ;[1 1 1] Update Flipbook visuals
          (`PaperFlipbookComponent.SetFlipbook` (`self.Sprite`) (break `/Game/SpaceShooter2DKit/Blueprints/Characters/Player/STR_PlayerShip` _returnvalue)))
        (:`then_1`
          ;[1 1 1] Update Flipbook location
          (`SceneComponent.K2_SetRelativeLocation` (`self.Sprite`) (`.Location_20_FFCD22FE4B4F7BA52B0C4087DE55596C` (break `/Game/SpaceShooter2DKit/Blueprints/Characters/Player/STR_PlayerShip` _returnvalue)) false true))
        (:`then_2`
          ;[1 1 1] Update Flipbook scale
          (`SceneComponent.SetRelativeScale3D` (`self.Sprite`) (`.Scale_23_768DFF224EAD7DDB4F0BE082CB0A54D5` (break `/Game/SpaceShooter2DKit/Blueprints/Characters/Player/STR_PlayerShip` _returnvalue))))
        (:`then_3`
          ;[1 1 1] Update left thruster location
          (`SceneComponent.K2_SetRelativeLocation` (`self.LeftThruster`) (`.LeftThrusterLocation_24_FA439BDE4A809EA72A1FFCB3261476C5` (break `/Game/SpaceShooter2DKit/Blueprints/Characters/Player/STR_PlayerShip` _returnvalue)) false true))
        (:`then_4`
          ;[1 1 1] Update right thruster location
          (`SceneComponent.K2_SetRelativeLocation` (`self.RightThruster`) (`.RightThrusterLocation_25_932A59074FF1C5172F1EDB8047A2CB70` (break `/Game/SpaceShooter2DKit/Blueprints/Characters/Player/STR_PlayerShip` _returnvalue)) false true))))
    (:`RowNotFound`
      ;[1 1 1] Print error when ship is not found
      (`KismetSystemLibrary.PrintString` "Selected Ship not found in DataTable"))))

(fn `SetWeaponType`
  (params (Index :type Integer))
  ;[1 1 1] Update Weapon Type Index
  (bind _output_get (set `self.WeaponTypeIndex` Index))
  ;[1 1 1] Get the weapon type from the Data Table
  (bind _returnvalue (`|GetDataTableRow` "/Game/SpaceShooter2DKit/Blueprints/Characters/Player/DT_PlayerWeaponTypes.DT_PlayerWeaponTypes" (`|GetArrayItem` (`self.WeaponTypeNames`) _output_get))
    (:`then`
      ;[1 1 1] Set the weapon type
      (set `self.CurrentWeaponType` _returnvalue))))

(fn `ToggleThrustersVisibility`
  (params (Visible :type Boolean))
  ;[1 1 1] Toggle visibility of left and right thruster
  (`SceneComponent.SetVisibility` (`self.LeftThruster`) Visible false)
  (`SceneComponent.SetVisibility` (`self.RightThruster`) Visible false))

(fn `UpgradeWeapon`
  (`self.ChangeWeapon` 1))

(fn `UserConstructionScript`
  ;[1 1 1] Call constructor script of BaseCharacter
  (`parent.UserConstructionScript`))