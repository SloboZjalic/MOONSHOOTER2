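; Enemy spawner for a 2D shooter that keeps the count of one enemy type in the level under a maximum.
; Activate starts a looping SpawnEnemy timer at the configured spawn rate, and Deactivate clears both that timer and any Activate timer.
; Each tick gathers all BP_BaseEnemy actors, filters them by the spawnee's type, and spawns another at the spawnee's scale if below the cap.
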(event `/Game/SpaceShooter2DKit/Blueprints/Spawners/BP_iSpawner.Activate`
  ;[1 1 1] Call SpawnEnemy to achive spawnees per second rate
  (`KismetSystemLibrary.K2_SetTimer` null "SpawnEnemy" (/ 1.0 (`self.SpawneesPerSecond`)) true))

(event `/Game/SpaceShooter2DKit/Blueprints/Spawners/BP_iSpawner.Deactivate`
  ;[1 1 1] Clears timers on activate
  (`KismetSystemLibrary.K2_ClearTimer` null "SpawnEnemy")
  (`KismetSystemLibrary.K2_ClearTimer` null "Activate"))

(event `SpawnEnemy`
  (bind (_spawneeclass_type _spawneeclass_scale) (break `/Game/SpaceShooter2DKit/Blueprints/Spawners/STR_EnemySpawnee` (`self.SpawneeClass`)))
  (bind _spawneeclass_type_2 (break `/Game/SpaceShooter2DKit/Blueprints/Spawners/STR_EnemySpawnee` (`self.SpawneeClass`)))
  ;[1 1 1] Get all enemies in level
  (bind _outactors (`GameplayStatics.GetAllActorsOfClass` "/Game/SpaceShooter2DKit/Blueprints/Characters/Enemies/BP_BaseEnemy.BP_BaseEnemy_C"))
  ;[1 1 1] Filter on spawnee type
  (bind _filteredenemies (`self.FilterOnType` _outactors _spawneeclass_type_2))
  ;[1 1 1] If true, spawn enemy
  (if (< (`KismetArrayLibrary.Array_Length` _filteredenemies) (`self.MaxSpawneesInLevel`))
    (`self.SpawnEnemyType` _spawneeclass_type _spawneeclass_scale)))

(fn `UserConstructionScript`)