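; BP_PickupSpawner randomly spawns pickups in the 2D space shooter while it is active.
; Activate starts a looping one-second timer on SpawnPickups, and Deactivate clears it.
; Each tick of that timer rolls every Spawnees entry independently, spawning its type at its configured scale on success.
; ApplySpawnChance converts the entry's spawns-per-minute rate into a per-second probability for a weighted random bool.
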(event `/Game/SpaceShooter2DKit/Blueprints/Spawners/BP_iSpawner.Activate`
  ;[1 1 1] On activate, start calling SpawnPickups every second
  (`KismetSystemLibrary.K2_SetTimer` null "SpawnPickups" 1.0 true))

(event `/Game/SpaceShooter2DKit/Blueprints/Spawners/BP_iSpawner.Deactivate`
  ;[1 1 1] Disable timer on deactivate
  (`KismetSystemLibrary.K2_ClearTimer` null "SpawnPickups"))

(event `SpawnPickups`
  ;[1 1 1] Loop through spawnable pickups
  (for _array_element (`self.Spawnees`)
    ;[1 1 1] Calculate whether to spawn on spawn chance
    (if (`self.ApplySpawnChance` (`.SpawnsPerMinute_8_84BB9319C04844174F10888E1CCA70A4` (break `/Game/SpaceShooter2DKit/Blueprints/Spawners/STR_PickupSpawnee` _array_element)))
      ;[1 1 1] If true, spawn pickup
      (`self.SpawnActor` (break `/Game/SpaceShooter2DKit/Blueprints/Spawners/STR_PickupSpawnee` _array_element) (`.Scale_11_CFAAAFFA7C4EE6D93F32319CBB3E3EF7` (break `/Game/SpaceShooter2DKit/Blueprints/Spawners/STR_PickupSpawnee` _array_element))))))

(fn `ApplySpawnChance`
  (params (`Spawns per Minute` :type "Float (double-precision)"))
  (returns (SpawnPickup :type Boolean))
  (return (`KismetMathLibrary.RandomBoolWithWeight` (/ `Spawns per Minute` 60.0))))

(fn `UserConstructionScript`
  (`parent.UserConstructionScript`))