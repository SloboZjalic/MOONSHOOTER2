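; Wave spawner for the 2D space shooter kit that repeatedly spawns waves of randomly chosen enemies.
; Activate starts a looping timer that picks a random Spawnees entry and passes its type and scale to SpawnEnemyType.
; Once SpawneesPerWave is reached, it resets the count and schedules Activate after WaveDelay.
; Deactivate clears only that pending Activate timer, so a wave in progress keeps spawning.
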(event `/Game/SpaceShooter2DKit/Blueprints/Spawners/BP_iSpawner.Activate`
  ;[1 1 1] Make sure Spawnees is not empty
  (if (> (`KismetArrayLibrary.Array_Length` (`self.Spawnees`)) 0)
    ;[1 1 1] Call SpawnEnemy every EnemyDelay
    (`KismetSystemLibrary.K2_SetTimer` null "SpawnEnemy" (`self.EnemyDelay`) true)
    (else
      (`KismetSystemLibrary.PrintString` "Add Spawnees to WaveSpawener"))))

(event `/Game/SpaceShooter2DKit/Blueprints/Spawners/BP_iSpawner.Deactivate`
  ;[1 1 1] Clear timer on deactivate
  (`KismetSystemLibrary.K2_ClearTimer` null "Activate"))

(event `SpawnEnemy`
  ;[1 1 1] Check wave not finished (current < max spawnees)
  (if (< (`self.CurrentSpawneeIndex`) (`self.SpawneesPerWave`))
    ;[1 1 1] If true, get spawnee properties and spawn actor
    (bind _actortospawn (`self.GetSpawnee`))
    (`self.SpawnEnemyType` (break `/Game/SpaceShooter2DKit/Blueprints/Spawners/STR_EnemySpawnee` _actortospawn) (`.Scale_5_F49C72B72D4D85DDA355C5A9587ED53E` (break `/Game/SpaceShooter2DKit/Blueprints/Spawners/STR_EnemySpawnee` _actortospawn)))
    ;[1 1 1] Increment current spawnee index
    (`/Engine/EditorBlueprintResources/StandardMacros.IncrementInt` (`self.CurrentSpawneeIndex`))
    (else
      ;[1 1 1] Else reset after wave
      (`self.ResetAfterWave`))))

(fn `GetSpawnee`
  (returns (ActorToSpawn :type "/Game/SpaceShooter2DKit/Blueprints/Spawners/STR_EnemySpawnee Structure"))
  (return (`|GetArrayItem` (`self.Spawnees`) (`KismetMathLibrary.RandomIntegerInRange` 0 (- (`KismetArrayLibrary.Array_Length` (`self.Spawnees`)) 1)))))

(fn `ResetAfterWave`
  ;[1 1 1] Clear SpawnEnemy timer
  (`KismetSystemLibrary.K2_ClearTimer` null "SpawnEnemy")
  ;[1 1 1] Reset index for next wave
  (set `self.CurrentSpawneeIndex` 0)
  ;[1 1 1] Wait wave delay and then call activate again
  (`KismetSystemLibrary.K2_SetTimer` null "Activate" (`self.WaveDelay`)))

(fn `UserConstructionScript`)