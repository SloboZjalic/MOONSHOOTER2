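; Base spawner Blueprint for a 2D space shooter that places actors and typed enemies at random points within a spawn area.
; When enabled, it activates after an initial delay on BeginPlay and can be deactivated through an event.
; SpawnEnemyType builds on the generic SpawnActor helper, creating a BP_BaseEnemy and switching its type if it is still valid.
; FilterOnType returns the enemies in an array that match a given type.
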(event `self.ReceiveBeginPlay`
  ;[1 1 1] If enabled, activate after initial delay
  (if (`self.Enabled`)
    (`KismetSystemLibrary.Delay` (`self.InitialDelay`))
    (`/Game/SpaceShooter2DKit/Blueprints/Spawners/BP_iSpawner.Activate`)))

(event `DeactivateSpawner`
  (`/Game/SpaceShooter2DKit/Blueprints/Spawners/BP_iSpawner.Deactivate`))

(fn `FilterOnType`
  (params (UnfilteredEnemies :type "Array of /Game/SpaceShooter2DKit/Blueprints/Characters/Enemies/BP_BaseEnemy Object Reference") (Type :type "/Game/SpaceShooter2DKit/Blueprints/Characters/Enemies/ENUM_EnemyType Enum" :default "NewEnumerator0"))
  (returns (FilteredEnemies :type "Array of /Game/SpaceShooter2DKit/Blueprints/Characters/Enemies/BP_BaseEnemy Object Reference"))
  (locals (Result :type "Array of /Game/SpaceShooter2DKit/Blueprints/Characters/Enemies/BP_BaseEnemy Object Reference"))
  ;[1 1 1] Loop through entries and check type
  (for _array_element UnfilteredEnemies
    ;[1 1 1] If matching type, add to result array
    (if (`/Game/SpaceShooter2DKit/Blueprints/Characters/Enemies/BP_BaseEnemy.HasType` _array_element Type)
      (`KismetArrayLibrary.Array_Add` (`local.Result`) _array_element)))
  ;[1 1 1] Return result array
  (return (`local.Result`)))

(fn `SpawnActor`
  (params (Class :type "Actor Class Reference") (Scale :type "Vector Structure"))
  (returns (SpawnedActor :type "Actor Object Reference"))
  (bind _spawnarea (`self.SpawnArea`))
  ;[1 1 1] Spawn actor of class in random location using given scale
  (bind _returnvalue (`|SpawnActorFromClass` Class (`KismetMathLibrary.MakeTransform` (`KismetMathLibrary.MakeVector` (`KismetMathLibrary.RandomFloatInRange` (.x (break `/Game/SpaceShooter2DKit/Blueprints/Spawners/STR_SpawnArea` _spawnarea)) (.x (`.MaximumCoordinates_13_72D42F28E14888D7781FD4858CDB8A28` (break `/Game/SpaceShooter2DKit/Blueprints/Spawners/STR_SpawnArea` _spawnarea)))) (`KismetMathLibrary.RandomFloatInRange` (.y (break `/Game/SpaceShooter2DKit/Blueprints/Spawners/STR_SpawnArea` _spawnarea)) (.y (`.MaximumCoordinates_13_72D42F28E14888D7781FD4858CDB8A28` (break `/Game/SpaceShooter2DKit/Blueprints/Spawners/STR_SpawnArea` _spawnarea)))) (`KismetMathLibrary.RandomFloatInRange` (.z (break `/Game/SpaceShooter2DKit/Blueprints/Spawners/STR_SpawnArea` _spawnarea)) (.z (`.MaximumCoordinates_13_72D42F28E14888D7781FD4858CDB8A28` (break `/Game/SpaceShooter2DKit/Blueprints/Spawners/STR_SpawnArea` _spawnarea))))) (struct) Scale) "Undefined" "OverrideRootScale" null null))
  (return _returnvalue))

(fn `SpawnEnemyType`
  (params (Type :type "/Game/SpaceShooter2DKit/Blueprints/Characters/Enemies/ENUM_EnemyType Enum" :default "NewEnumerator0") (Scale :type "Vector Structure"))
  (returns (Enemy :type "/Game/SpaceShooter2DKit/Blueprints/Characters/Enemies/BP_BaseEnemy Object Reference"))
  (locals (SpawnedEnemy :type "/Game/SpaceShooter2DKit/Blueprints/Characters/Enemies/BP_BaseEnemy Object Reference"))
  ;[1 1 1] Spawn BaseEnemy actor and save in variable
  (bind _spawnedactor (`self.SpawnActor` "/Game/SpaceShooter2DKit/Blueprints/Characters/Enemies/BP_BaseEnemy.BP_BaseEnemy_C" Scale))
  (bind _asbp_base_enemy (cast `/Game/SpaceShooter2DKit/Blueprints/Characters/Enemies/BP_BaseEnemy` _spawnedactor))
  (bind _output_get (set `local.SpawnedEnemy` _asbp_base_enemy))
  ;[1 1 1] If enemy is still valid (alive), change its type
  (`/Engine/EditorBlueprintResources/StandardMacros.IsValid` _output_get
    (:`Is Valid`
      (`/Game/SpaceShooter2DKit/Blueprints/Characters/Enemies/BP_BaseEnemy.ChangeType` (`local.SpawnedEnemy`) Type)
      ;[1 1 1] Return enemy
      (return (`local.SpawnedEnemy`)))))

(fn `UserConstructionScript`)