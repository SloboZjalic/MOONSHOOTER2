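; Player controller for the 2D space shooter kit that owns the HUD and manages pause, game over and level complete menus.
; On BeginPlay it creates BP_HUD, adds it to the viewport and sets game-only input.
; The Pause input pauses the game, shows the cursor and focuses the resume button in UI-only mode, while UnpauseGame reverses this.
; End-of-level functions show their HUD menus and focus the main menu button.
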(event `self.ReceiveBeginPlay`
  ;[1 1 1] Add HUD to viewport
  (bind _returnvalue (`|CreateWidget` "/Game/SpaceShooter2DKit/Blueprints/UI/BP_HUD.BP_HUD_C"))
  (bind _output_get (set `self.HUD` _returnvalue))
  (`UserWidget.AddToViewport` _output_get 0)
  (`WidgetBlueprintLibrary.SetInputMode_GameOnly` self))

(event `InputAction|Pause`
  (params (Key :type "Key Structure"))
  (:`Pressed`
    ;[1 1 1] Pause the game
    (`self.PauseGame`)))

(fn `PauseGame`
  ;[1 1 1] Show pause menu
  (bind _hud (`self.HUD`)
    (:`then`
      (`/Game/SpaceShooter2DKit/Blueprints/UI/BP_HUD.ShowPauseMenu` _hud)
      ;[1 1 1] Set game paused variable
      (bind _returnvalue (`GameplayStatics.SetGamePaused` true))
      ;[1 1 1] Show the mouse cursor
      (set `self.bShowMouseCursor` _returnvalue)
      ;[1 1 1] Set input UI only and focus resume button
      (`WidgetBlueprintLibrary.SetInputMode_UIOnlyEx` self (`/Game/SpaceShooter2DKit/Blueprints/UI/BP_HUD.ResumeButton` (`self.HUD`))))
    (:`else`)))

(fn `ShowGameOverMenu`
  (`/Game/SpaceShooter2DKit/Blueprints/UI/BP_HUD.ShowGameOverMenu` (`self.HUD`))
  ;[1 1 1] Show the mouse cursor
  (set `self.bShowMouseCursor` true)
  ;[1 1 1] Set input UI only and focus MainMenu button
  (`WidgetBlueprintLibrary.SetInputMode_UIOnlyEx` self (`/Game/SpaceShooter2DKit/Blueprints/UI/BP_HUD.MainMenuButton` (`self.HUD`))))

(fn `ShowLevelCompleteMenu`
  (`/Game/SpaceShooter2DKit/Blueprints/UI/BP_HUD.ShowLevelCompleteMenu` (`self.HUD`))
  ;[1 1 1] Show the mouse cursor
  (set `self.bShowMouseCursor` true)
  ;[1 1 1] Set input UI only and focus MainMenu button
  (`WidgetBlueprintLibrary.SetInputMode_UIOnlyEx` self (`/Game/SpaceShooter2DKit/Blueprints/UI/BP_HUD.MainMenuButton` (`self.HUD`))))

(fn `UnpauseGame`
  ;[1 1 1] Unpause the game
  (`GameplayStatics.SetGamePaused` false)
  ;[1 1 1] Hide mouse cursor
  (set `self.bShowMouseCursor` false)
  ;[1 1 1] Set input Game only
  (`WidgetBlueprintLibrary.SetInputMode_GameOnly` self))

(fn `UserConstructionScript`)