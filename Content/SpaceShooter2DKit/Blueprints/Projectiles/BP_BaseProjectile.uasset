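; BP_BaseProjectile is the base projectile Blueprint in the SpaceShooter2DKit, providing straight or homing flight.
; Its construction script calls InitializeMovement, which sets the ProjectileMovement component's local-space velocity from Direction and its initial speed from Speed.
; EnableHoming switches that component to homing with the HomingAcceleration magnitude, tracking the given target's capsule component.
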(fn `EnableHoming`
  (params (Target :type "/Game/SpaceShooter2DKit/Blueprints/Characters/BP_BaseCharacter Object Reference"))
  (`|ExecutionSequence`
    (:`then_0`
      ;[1 1 1] Set homing projectile
      (set `ProjectileMovementComponent.bIsHomingProjectile` true (`self.ProjectileMovement`)))
    (:`then_1`
      ;[1 1 1] Set homing acceleration magnitude
      (set `ProjectileMovementComponent.HomingAccelerationMagnitude` (`self.HomingAcceleration`) (`self.ProjectileMovement`)))
    (:`then_2`
      ;[1 1 1] Set homing target to target collision capsule
      (set `ProjectileMovementComponent.HomingTargetComponent` (`Character.CapsuleComponent` Target) (`self.ProjectileMovement`)))))

(fn `InitializeMovement`
  (bind _projectilemovement (`self.ProjectileMovement`))
  (`|ExecutionSequence`
    (:`then_0`
      ;[1 1 1] Set initial direction
      (`ProjectileMovementComponent.SetVelocityInLocalSpace` _projectilemovement (`self.Direction`)))
    (:`then_1`
      ;[1 1 1] Set initial speed
      (set `ProjectileMovementComponent.InitialSpeed` (`self.Speed`) _projectilemovement))))

(fn `UserConstructionScript`
  (`self.InitializeMovement`))