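; BP_SuicideAI is an AI controller that steers an enemy toward the player, by its name as a suicide attacker.
; On possess it caches the pawn as a BP_BaseEnemy.
; Each tick, while that enemy is alive and higher in Z than the player, it moves directly at the player character without pathfinding.
; Otherwise it stops the AI move, leaving the enemy to its default movement.
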(event `self.ReceivePossess`
  (params (PossessedPawn :type "Pawn Object Reference"))
  ;[1 1 1] Set controlled pawn variable
  (bind _asbp_base_enemy (cast `/Game/SpaceShooter2DKit/Blueprints/Characters/Enemies/BP_BaseEnemy` PossessedPawn))
  (set `self.ControlledPawn` _asbp_base_enemy))

(event `self.ReceiveTick`
  (params (DeltaSeconds :type "Float (single-precision)"))
  ;[1 1 1] If above player and controlled pawn alive, move to player. Else use default movement
  (if (and (`self.IsAbovePlayer`) (not (`/Game/SpaceShooter2DKit/Blueprints/Characters/BP_BaseCharacter.IsDead` (`self.ControlledPawn`))))
    (`self.MoveToActor` (`GameplayStatics.GetPlayerCharacter` 0) -1.0 true false true null)
    (else
      (`self.StopMovement`))))

(fn `IsAbovePlayer`
  (returns (AbovePlayer :type Boolean))
  (bind (_returnvalue_x _returnvalue_y _returnvalue_z) (`KismetMathLibrary.BreakVector` (`self.K2_GetActorLocation` (`self.ControlledPawn`))))
  (bind (_returnvalue_x_2 _returnvalue_y_2 _returnvalue_z_2) (`KismetMathLibrary.BreakVector` (`self.K2_GetActorLocation` (`GameplayStatics.GetPlayerCharacter` 0))))
  (return (> _returnvalue_z _returnvalue_z_2)))

(fn `UserConstructionScript`)